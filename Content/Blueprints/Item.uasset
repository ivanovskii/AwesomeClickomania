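; Item is a clickable colored sphere piece on a puzzle board that reports clicks to the Board.
; BeginPlay sets the sphere's blue, red or green material from its Color, and an Animation event moves the sphere component to a given world location.
; A click calls Board.OnItemClick, then checks win or lose, showing the matching screen, pausing and switching to UI-only input, with lose checked first.
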(event Custom|Event%20Animation
  (params (NewLoc :type Vector))
  (Components|MoveComponentTo (Variables|Default|GetSphere) (- NewLoc (Transformation|GetActorLocation)) "0, 0, 0" false false 0.2 false))

(event EventBeginPlay
  (bind _sphere (Variables|Default|GetSphere))
  (switch int (Variables|Default|GetColor)
    (:0
      (Rendering|Material|SetMaterial _sphere 0 "/Game/Materials/Blue.Blue"))
    (:1
      (Rendering|Material|SetMaterial _sphere 0 "/Game/Materials/Red.Red"))
    (:2
      (Rendering|Material|SetMaterial _sphere 0 "/Game/Materials/Green.Green"))))

(event MouseInput|EventActorOnClicked
  (params (ButtonPressed :type Key%20Structure :default "None"))
  (Default|OnItemClick (Variables|Default|GetBoard) self)
  (bind (_iswin _islose) (Default|CheckWinorLose (Variables|Default|GetBoard)))
  (if _islose
    (bind _returnvalue (UserInterface|CreateWidget "/Game/Blueprints/LoseScreen.LoseScreen_C"))
    (UserInterface|Viewport|AddtoViewport _returnvalue 0)
    (Game|SetGamePaused true)
    (Input|SetInputModeUIOnly (Game|GetPlayerController 0) 0 "DoNotLock")
    (elif _iswin
      (bind _returnvalue_2 (UserInterface|CreateWidget "/Game/Blueprints/WinScreen.WinScreen_C"))
      (UserInterface|Viewport|AddtoViewport _returnvalue_2 0)
      (Game|SetGamePaused true)
      (Input|SetInputModeUIOnly (Game|GetPlayerController 0) 0 "DoNotLock"))))

(fn ConstructionScript)