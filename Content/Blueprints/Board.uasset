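; Board actor for a SameGame-style puzzle that spawns a checkered square grid of cells with randomly colored items, stored in an IntPoint-keyed map.
; Clicking an item runs a breadth-first flood fill (Paint) to find its same-color group and destroys groups of two or more.
; Remaining items then drop into gaps and empty columns are closed up, with animated moves.
; CheckWinOrLose reports a win on an empty board, a loss when only singles remain.
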(event EventBeginPlay
  (CallFunction|SpawnCells)
  (Components|DestroyComponent (Variables|Default|GetPlaceholder))
  (CallFunction|SpawnItems))

(fn ConstructionScript)

(fn SpawnCell
  (params (XY :type Int%20Point%20Structure))
  (bind (_x _y) (Utilities|Struct|BreakIntPoint XY))
  (bind _location (CallFunction|XYtoLocation XY))
  (bind _returnvalue (Game|SpawnActorfromClass "/Game/Blueprints/Cell.Cell_C" (Math|Transform|MakeTransform _location) "Undefined" 0 0))
  (Default|SetMaterial _returnvalue (== (Math|Integer|%(Integer) (+ _x _y) 2) 0))
  (return _returnvalue))

(fn SpawnCells
  (bind _xy (Utilities|EnumerateCoords)
    (:LoopBody
      (CallFunction|SpawnCell _xy))))

(fn XYtoLocation
  (params (XY :type Int%20Point%20Structure))
  (bind (_x _y) (Utilities|Struct|BreakIntPoint XY))
  (return (- (* (Math|Vector|MakeVector (Math|Conversions|ToFloat(Integer) _x) (Math|Conversions|ToFloat(Integer) _y) 5.0) (Variables|Default|GetCellSize)) (- (/ (* (Variables|Default|GetSize) (Variables|Default|GetCellSize)) 2.0) (/ (Variables|Default|GetCellSize) 2.0)))))

(fn SpawnItems
  (bind _xy (Utilities|EnumerateCoords)
    (:LoopBody
      (bind _location (CallFunction|XYtoLocation _xy))
      (bind _returnvalue (Game|SpawnActorfromClass "/Game/Blueprints/Item.Item_C" (Math|Conversions|ToTransform(Vector) _location) "Undefined" 0 (Math|Random|RandomIntegerinRange 0 2) self 0))
      (Utilities|Map|Add (Variables|Default|GetItems) _xy _returnvalue))))

(fn OnItemClick
  (params (Item :type Item%20Object%20Reference))
  (bind _items (Variables|Default|GetItems))
  (bind _xy (CallFunction|ItemtoXY Item))
  (bind _paintedarray (CallFunction|Paint _xy))
  (if (> (Utilities|Array|Length _paintedarray) 1)
    (for _array_element _paintedarray
      (Actor|DestroyActor (.Value (Utilities|Map|Find _items _array_element)))
      (Utilities|Map|Remove _items _array_element))
    (CallFunction|DropItems)))

(fn ItemtoXY
  (params (Item :type Item%20Object%20Reference))
  (bind _xy (Utilities|EnumerateCoords)
    (:LoopBody
      (if (== (.Value (Utilities|Map|Find (Variables|Default|GetItems) _xy)) Item)
        (LocalVariables|SetResult _xy)))
    (:Complete
      (return (LocalVariables|GetResult)))))

(fn Paint
  (params (XY :type Int%20Point%20Structure))
  (bind _paintmap (LocalVariables|GetPaintMap))
  (bind _queue (LocalVariables|GetQueue))
  (bind _output_get (LocalVariables|SetOurXY XY))
  (LocalVariables|SetOurColor (Variables|/Game/Blueprints/Item.Item_C|GetColor (.Value (Utilities|Map|Find (Variables|Default|GetItems) _output_get))))
  (bind _xy (Utilities|EnumerateCoords)
    (:LoopBody
      (Utilities|Map|Add (LocalVariables|GetPaintMap) _xy (LocalVariables|Getinf)))
    (:Complete
      (Utilities|Array|Add (LocalVariables|GetQueue) (LocalVariables|GetOurXY))
      (Utilities|Map|Add (LocalVariables|GetPaintMap) (LocalVariables|GetOurXY) 0)
      (while (Utilities|Array|IsNotEmpty (LocalVariables|GetQueue))
        (bind _output_get_2 (LocalVariables|SetOurXY (Utilities|Array|Get(acopy) _queue)))
        (Utilities|Array|RemoveIndex _queue)
        (bind _neighboorxy (Utilities|EnumerateNeighboursOfColor _output_get_2 (LocalVariables|GetOurColor))
          (:Loop
            (if (> (.Value (Utilities|Map|Find _paintmap _neighboorxy)) (+ (.Value (Utilities|Map|Find _paintmap (LocalVariables|GetOurXY))) 1))
              (Utilities|Map|Add (LocalVariables|GetPaintMap) _neighboorxy (+ (.Value (Utilities|Map|Find _paintmap (LocalVariables|GetOurXY))) 1))
              (Utilities|Array|Add (LocalVariables|GetQueue) _neighboorxy)))))
      (bind _xy_2 (Utilities|EnumerateCoords)
        (:LoopBody
          (if (< (.Value (Utilities|Map|Find (LocalVariables|GetPaintMap) _xy_2)) (LocalVariables|Getinf))
            (Utilities|Array|Add (LocalVariables|GetResult) _xy_2)))
        (:Complete
          (return (LocalVariables|GetResult)))))))

(fn IsColumnEmpty
  (params (ColInd :type Integer))
  (for _index (range 0 (- (Variables|Default|GetSize) 1))
    (bind _empty (CallFunction|IsCellEmpty (Utilities|Struct|MakeIntPoint ColInd _index)))
    (if (not _empty)
      (LocalVariables|SetColCounter (+ (LocalVariables|GetColCounter) 1))))
  (return (== (LocalVariables|GetColCounter) 0)))

(fn IsCellEmpty
  (params (XY :type Int%20Point%20Structure))
  (bind (_x _y) (Utilities|Struct|BreakIntPoint XY))
  (bind _size (Variables|Default|GetSize))
  (return (Math|Boolean|ANDBoolean (not (.ReturnValue (Utilities|Map|Find (Variables|Default|GetItems) XY))) (Math|Integer|InRange(Integer) _x 0 _size true false) (Math|Integer|InRange(Integer) _y 0 _size true false))))

(fn TryDropDown
  (bind _xy (Utilities|EnumerateCoords)
    (:LoopBody
      (bind _output_get (LocalVariables|SetOldXY _xy))
      (bind _output_get_2 (LocalVariables|SetNewXY (+ _output_get (Class|KismetMathLibrary|IntPointUp))))
      (if (.ReturnValue (Utilities|Map|Find (Variables|Default|GetItems) _output_get))
        (bind _empty (CallFunction|IsCellEmpty _output_get_2))
        (if _empty
          (bind _output_get_3 (LocalVariables|SetItem (.Value (Utilities|Map|Find (Variables|Default|GetItems) (LocalVariables|GetOldXY)))))
          (Utilities|Map|Add (Variables|Default|GetItems) (LocalVariables|GetNewXY) _output_get_3)
          (Utilities|Map|Remove (Variables|Default|GetItems) (LocalVariables|GetOldXY))
          (bind _location (CallFunction|XYtoLocation (LocalVariables|GetNewXY)))
          (Default|EventAnimation (LocalVariables|GetItem) _location)
          (LocalVariables|SetResult true))))
    (:Complete
      (return (LocalVariables|GetResult)))))

(fn TryDropLeft
  (params (CurrColInd :type Integer) (NewColInd :type Integer))
  (bind _items (Variables|Default|GetItems))
  (for _index (range 0 (- (Variables|Default|GetSize) 0))
    (bind _output_get (LocalVariables|SetOldXY (Utilities|Struct|MakeIntPoint CurrColInd _index)))
    (LocalVariables|SetNewXY (Utilities|Struct|MakeIntPoint NewColInd _index))
    (if (.ReturnValue (Utilities|Map|Find (Variables|Default|GetItems) _output_get))
      (bind _output_get_2 (LocalVariables|SetItem (.Value (Utilities|Map|Find _items (LocalVariables|GetOldXY)))))
      (Utilities|Map|Add _items (LocalVariables|GetNewXY) _output_get_2)
      (Utilities|Map|Remove (Variables|Default|GetItems) (LocalVariables|GetOldXY))
      (bind _location (CallFunction|XYtoLocation (LocalVariables|GetNewXY)))
      (Default|EventAnimation (LocalVariables|GetItem) _location))))

(fn DropItems
  (while (LocalVariables|GetAreColumnsDroppable)
    (bind _succes (CallFunction|TryDropDown))
    (LocalVariables|SetAreColumnsDroppable _succes))
  (bind _colind (Utilities|EnumerateColumns)
    (:Loop%20Body
      (bind _isempty (CallFunction|IsColumnEmpty _colind))
      (if _isempty
        (bind (_isfind _notemptycolind) (CallFunction|NotEmptyColumn _colind))
        (if _isfind
          (CallFunction|TryDropLeft _notemptycolind _colind))))))

(fn NotEmptyColumn
  (params (EmptyColInd :type Integer))
  (if (== EmptyColInd 0)
    (return (LocalVariables|Getis_find) 0)
    (else
      (bind _index (Utilities|FlowControl|ForLoopwithBreak 0 EmptyColInd :!label _label)
        (:LoopBody
          (bind _isempty (CallFunction|IsColumnEmpty (- EmptyColInd _index)))
          (if (not _isempty)
            (LocalVariables|Setis_find true)
            (goto _label Break)))
        (:Completed
          (return (LocalVariables|Getis_find) (- EmptyColInd _index)))))))

(fn CheckWinorLose
  (bind _xy (Utilities|EnumerateCoords)
    (:LoopBody
      (if (.ReturnValue (Utilities|Map|Find (Variables|Default|GetItems) _xy))
        (LocalVariables|SetAreThereNonEmptyCells true)
        (bind _paintedarray (CallFunction|Paint _xy))
        (if (> (Utilities|Array|Length _paintedarray) 1)
          (LocalVariables|SetAreThereNonSingleCells true))))
    (:Complete
      (if (LocalVariables|GetAreThereNonEmptyCells)
        (if (not (LocalVariables|GetAreThereNonSingleCells))
          (return false true))
        (else
          (return true false))))))